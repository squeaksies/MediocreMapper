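; BP_strobe is a timeline marker actor for a rhythm-game note track, shown as a bar colored by its Type.
; UpdateStrobe, run from the construction script, places the actor by Time and stretches the mesh by Duration, both scaled by note separation, with Line setting the sideways offset.
; Type selects a bomb, blue ghost-note or red ghost-note material.
; GetProperties packs Time, Line, Type and Duration into an Obstacle struct.
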(event Custom|UpdateStrobe
  (bind _meshroot (Variables|Default|GetMeshRoot))
  (Transformation|SetWorldScale3D _meshroot (Math|Vector|MakeVector 0.5 (* (Variables|Default|GetDuration) (/ (CallFunction|GetNoteSep) 1e+02)) 0.5))
  (Transformation|SetRelativeLocation _meshroot (Math|Vector|MakeVector (* (Variables|Default|GetLine) 5e+01) 0.0 0.0) false false)
  (Rendering|Material|SetMaterial (Variables|Default|GetMesh) 0 (Utilities|Select :Index (Variables|Default|GetType) :Option%200 "/Game/Materials/M_bomb.M_bomb" :Option%201 "/Game/Materials/M_ghost_note_blue.M_ghost_note_blue" :Option%202 "/Game/Materials/M_ghost_note_blue.M_ghost_note_blue" :Option%203 "/Game/Materials/M_ghost_note_blue.M_ghost_note_blue" :Option%204 "/Game/Materials/M_bomb.M_bomb" :Option%205 "/Game/Materials/M_ghost_note_red.M_ghost_note_red" :Option%206 "/Game/Materials/M_ghost_note_red.M_ghost_note_red" :Option%207 "/Game/Materials/M_ghost_note_red.M_ghost_note_red"))
  (Transformation|SetActorRelativeLocation (Math|Vector|MakeVector 0.0 (* (* (CallFunction|GetNoteSep) (Variables|Default|GetTime)) -1.0) 0.0)))

(fn ConstructionScript
  (CallFunction|UpdateStrobe))

(fn GetProperties
  (return (Utilities|Struct|MakeStructObstacle (Variables|Default|GetTime) (Variables|Default|GetLine) (Variables|Default|GetType) (Variables|Default|GetDuration))))