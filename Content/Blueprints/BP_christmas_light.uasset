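; Christmas light Blueprint that continuously cycles the "Color" material parameter on its mesh.
; On construction, it picks a random RGB channel and gives it a random starting intensity, leaving the others at zero.
; Each Tick applies the color, then ramps the active channel by a fixed, frame-rate-dependent step.
; At either limit it flips the ramp direction and moves to the next channel in red, blue, green order.
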(event Custom|setFirstColor
  (bind _returnvalue (Math|Random|RandomFloat))
  (bind _output_get (Variables|Default|SetchangeColor (Math|Random|RandomInteger 3)))
  (bind _output_get_2 (Variables|Default|SetcurrentColor (Math|Vector|MakeVector (Math|Float|SelectFloat _returnvalue 0.0 (== _output_get 0)) (Math|Float|SelectFloat _returnvalue 0.0 (== _output_get 1)) (Math|Float|SelectFloat _returnvalue 0.0 (== _output_get 2)))))
  (Rendering|Material|SetVectorParameterValueonMaterials (Variables|Default|GetEventMesh) "Color" _output_get_2))

(event EventTick
  (params (DeltaSeconds :type Float%20%28single-precision%29))
  (Rendering|Material|SetVectorParameterValueonMaterials (Variables|Default|GetEventMesh) "Color" (Variables|Default|GetcurrentColor))
  (switch int (Variables|Default|GetchangeColor)
    (:0
      (bind _output_get (Variables|Default|SetcurrentColor (Math|Vector|MakeVector (+ (.X (Math|Vector|BreakVector (Variables|Default|GetcurrentColor))) (select (Variables|Default|Getincreasing) 0.01 -0.01)) (.Y (Math|Vector|BreakVector (Variables|Default|GetcurrentColor))) (.Z (Math|Vector|BreakVector (Variables|Default|GetcurrentColor))))))
      (if (Variables|Default|Getincreasing)
        (if (>= (.X (Math|Vector|BreakVector _output_get)) 1.0)
          (Variables|Default|SetchangeColor 2)
          (Variables|Default|Setincreasing false))
        (elif (<= (.X (Math|Vector|BreakVector _output_get)) 0.0)
          (Variables|Default|SetchangeColor 2)
          (Variables|Default|Setincreasing true))))
    (:1
      (bind _output_get_2 (Variables|Default|SetcurrentColor (Math|Vector|MakeVector (.X (Math|Vector|BreakVector (Variables|Default|GetcurrentColor))) (+ (.Y (Math|Vector|BreakVector (Variables|Default|GetcurrentColor))) (select (Variables|Default|Getincreasing) 0.01 -0.01)) (.Z (Math|Vector|BreakVector (Variables|Default|GetcurrentColor))))))
      (if (Variables|Default|Getincreasing)
        (if (>= (.Y (Math|Vector|BreakVector _output_get_2)) 1.0)
          (Variables|Default|SetchangeColor 0)
          (Variables|Default|Setincreasing false))
        (elif (<= (.Y (Math|Vector|BreakVector _output_get_2)) 0.0)
          (Variables|Default|SetchangeColor 0)
          (Variables|Default|Setincreasing true))))
    (:2
      (bind _output_get_3 (Variables|Default|SetcurrentColor (Math|Vector|MakeVector (.X (Math|Vector|BreakVector (Variables|Default|GetcurrentColor))) (.Y (Math|Vector|BreakVector (Variables|Default|GetcurrentColor))) (+ (.Z (Math|Vector|BreakVector (Variables|Default|GetcurrentColor))) (select (Variables|Default|Getincreasing) 0.01 -0.01)))))
      (if (Variables|Default|Getincreasing)
        (if (>= (.Z (Math|Vector|BreakVector _output_get_3)) 1.0)
          (Variables|Default|SetchangeColor 1)
          (Variables|Default|Setincreasing false))
        (elif (<= (.Z (Math|Vector|BreakVector _output_get_3)) 0.0)
          (Variables|Default|SetchangeColor 1)
          (Variables|Default|Setincreasing true))))))

(fn ConstructionScript
  (CallFunction|SetFirstColor))